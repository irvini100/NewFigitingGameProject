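; Game mode for a local two-player fighting match that manages player spawning, rounds and match wins.
; BeginPlay spawns characters chosen in MyGameInstance at P1/P2 tagged starts, creates a second controller, cross-links opponents and adds the HUD.
; Round events toggle timer and attacks, while Tick's timer check calls TimeOver to award the round by higher health.
; ResetMatchValues clears scores and respawns both players; DetermineMatchWinner compares wins against NumRounds.
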(event `ResetMatchValues`
  (bind _player1 (`self.player1`))
  (bind _player2 (`self.player2`))
  (set `FightingGameProjectCharacter.roundsWon` 0 (`self.player1`))
  (set `FightingGameProjectCharacter.roundsWon` 0 (`self.player2`))
  (bind _foundwidgets (`WidgetBlueprintLibrary.GetAllWidgetsOfClass` "/Game/BaseGMHud.BaseGMHud_C"))
  (`/Game/BaseGMHud.UpdateRoundCircles` _foundwidgets 0 0)
  (`/Game/BaseGMHud.UpdateRoundCircles` (`|GetArrayItem` _foundwidgets) 1 0)
  (`self.K2_DestroyActor` (`self.player1`))
  (`self.K2_DestroyActor` (`self.player2`))
  (set `self.roundTime` 99.0)
  (bind _asmy_game_instance (cast `MyGameInstance` (`GameplayStatics.GetGameInstance`) :!label _label))
  (bind _output_get (set `self.GameInstanceReference` _asmy_game_instance))
  (set `MyGameInstance.isDeviceForMultipleplayers` true _output_get)
  (bind _outactors (`GameplayStatics.GetAllActorsOfClass` "/Script/Engine.PlayerStart"))
  (for _array_element _outactors
    (`self.SpawnPlayers` _array_element))
  (if (`KismetSystemLibrary.IsValid` (`self.player1`))
    (if (`KismetSystemLibrary.IsValid` (`self.player2`))
      (set `FightingGameProjectCharacter.otherPlayer` _player2 _player1)
      (set `FightingGameProjectCharacter.otherPlayer` _player1 _player2)
      (set `FightingGameProjectCharacter.isFlipped` true _player2)
      (bind _returnvalue (`|CreateWidget` "/Game/BaseGMHud.BaseGMHud_C" (`GameplayStatics.GetPlayerController` 0)))
      (`UserWidget.AddToViewport` _returnvalue 0))))

(event `self.ReceiveBeginPlay`
  (goto _label))

(event `self.ReceiveTick`
  (params (DeltaSeconds :type "Float (single-precision)"))
  (bind _returnvalue (- (`self.roundTime`) DeltaSeconds))
  (if (`self.isTimerActive`)
    (if (== _returnvalue 0.0)
      (set `self.roundTime` _returnvalue)
      (else
        (set `self.roundTime` 0.0)
        (`self.TimeOver`)))))

(event `Round Start`
  (set `self.isTimerActive` true)
  (set `FightingGameProjectCharacter.canAttack` true (`self.player1`))
  (set `FightingGameProjectCharacter.canAttack` true (`self.player2`))
  (set `FightingGameProjectCharacter.playerHealth` 1.0 (`self.player1`))
  (set `FightingGameProjectCharacter.playerHealth` 1.0 (`self.player2`)))

(event `Round End`
  (set `self.isTimerActive` false)
  (set `FightingGameProjectCharacter.canAttack` false (`self.player1`))
  (set `FightingGameProjectCharacter.canAttack` false (`self.player2`)))

(fn `DetermineCharacter`
  (params (SpawnTransform :type "Transform Structure") (Actor :type "Actor Object Reference") (PlayerIndex :type Integer))
  (returns (CharacterReference :type "FightingGameProjectCharacter Object Reference") (NewParam :type Boolean))
  (bind _asmy_game_instance (cast `MyGameInstance` (`GameplayStatics.GetGameInstance`)))
  (switch `int` PlayerIndex
    (:`Default`
      (switch `ECharacterClass` (`MyGameInstance.P1characterClass` _asmy_game_instance) :!label _label
        (:`VE_DEFAULT`
          _)
        (:`VE_XBot`
          (bind _returnvalue (`|SpawnActorFromClass` "/Game/AllCharacters/YBot/XBot_BP.XBot_BP_C" SpawnTransform "Undefined" "OverrideRootScale" Actor null :!label _label_2))
          (return _returnvalue false))))
    (:`0`
      (goto _label))
    (:`1`
      (switch `ECharacterClass` (`MyGameInstance.P2characterClass` _asmy_game_instance)
        (:`VE_DEFAULT`
          _)
        (:`VE_XBot`
          (goto _label_2)))))
  (bind _returnvalue_2 (`|SpawnActorFromClass` "/Game/SideScrollerCPP/Blueprints/SideScrollerCharacter.SideScrollerCharacter_C" SpawnTransform "Undefined" "OverrideRootScale" Actor null))
  (`KismetSystemLibrary.PrintString` "Hello")
  (return _returnvalue_2 false))

(fn `DetermineMatchWinner`
  (returns (WinnerIndex :type Integer))
  (if (>= (`FightingGameProjectCharacter.roundsWon` (`self.player1`)) (`self.numRounds`))
    (`FightingGameProjectCharacter.WinMatch` (`self.player1`))
    (return 0)
    (elif (>= (`FightingGameProjectCharacter.roundsWon` (`self.player2`)) (`self.numRounds`))
      (`FightingGameProjectCharacter.WinMatch` (`self.player2`))
      (return 1)
      (else
        (return -1)))))

(fn `SpawnPlayers`
  (params (Object :type "Actor Object Reference"))
  (bind _returnvalue (`self.GetTransform` Object))
  (bind _asplayer_start (cast `PlayerStart` Object))
  (bind _playerstarttag (`PlayerStart.PlayerStartTag` _asplayer_start))
  (if (== "P1" _playerstarttag)
    (bind _characterreference (`self.DetermineCharacter` (`self.GetTransform` Object) Object))
    (set `self.player1` _characterreference)
    (`Controller.Possess` (`GameplayStatics.GetPlayerController` 0) _characterreference)
    (elif (== _playerstarttag "P2")
      (bind _returnvalue_2 (`|SpawnActorFromClass` "/Script/FightingGameProject.MyPlayerController" _returnvalue "Undefined" "OverrideRootScale" null null))
      (bind _characterreference_2 (`self.DetermineCharacter` _returnvalue Object 1))
      (set `self.player2` _characterreference_2)
      (`Controller.Possess` _returnvalue_2 _characterreference_2)
      (`KismetSystemLibrary.PrintString` "It's working"))))

(fn `TimeOver`
  (if (> (`FightingGameProjectCharacter.playerHealth` (`self.player1`)) (`FightingGameProjectCharacter.playerHealth` (`self.player2`)))
    (`FightingGameProjectCharacter.WinRound` (`self.player1`))
    (set `self.roundTime` 99.0)
    (elif (< (`FightingGameProjectCharacter.playerHealth` (`self.player1`)) (`FightingGameProjectCharacter.playerHealth` (`self.player2`)))
      (`FightingGameProjectCharacter.WinRound` (`self.player2`))
      (set `self.roundTime` 99.0))))

(fn `UserConstructionScript`)