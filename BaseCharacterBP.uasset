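; Base character Blueprint for a fighting game, providing hurtbox setup and second-player keyboard control.
; On BeginPlay it spawns a hurtbox actor attached to and owned by itself, and caches the game mode's Player2 unless it is that character.
; Player 2 jump, attack and movement inputs received here are forwarded to the cached character's P2Keyboard functions, so one character's input drives the other.
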(event `self.ReceiveBeginPlay`
  (bind _asfighting_game_project_game_mode (cast `FightingGameProjectGameMode` (`GameplayStatics.GetGameMode`)))
  (bind _output_get (set `self.GameModeReference` _asfighting_game_project_game_mode))
  (bind _player2 (`FightingGameProjectGameMode.player2` _output_get))
  (if (not (== _player2 self))
    (bind _output_get_2 (set `self.Player2 References` _player2)))
  (bind _returnvalue (`|SpawnActorFromClass` "/Game/HurtboxActor_BP.HurtboxActor_BP_C" (`self.GetTransform` (`CharacterMovementComponent.GetCharacterOwner` (`self.CharacterMovement`))) "Undefined" "OverrideRootScale" _output_get_2 null))
  (bind _output_get_3 (set `self.hurtbox` _returnvalue))
  (`self.K2_AttachToActor` _output_get_3 self "None" "SnapToTarget" "SnapToTarget" "SnapToTarget" true)
  (`self.SetOwner` _returnvalue self))

(event `InputAction|JumpP2`
  (params (Key :type "Key Structure"))
  (bind _player2_references (`self.Player2 References`))
  (bind _player2_references_2 (`self.Player2 References`))
  (:`Pressed`
    (`/Engine/EditorBlueprintResources/StandardMacros.IsValid` _player2_references
      (:`Is Valid`
        (`self.P2KeyboardJump` _player2_references))))
  (:`Released`
    (`/Engine/EditorBlueprintResources/StandardMacros.IsValid` _player2_references_2
      (:`Is Valid`
        (`self.P2KeyboardStopJumping` _player2_references_2)))))

(event `InputAction|Attack1P2`
  (params (Key :type "Key Structure"))
  (bind _player2_references (`self.Player2 References`))
  (:`Pressed`
    (`/Engine/EditorBlueprintResources/StandardMacros.IsValid` _player2_references
      (:`Is Valid`
        (`self.P2KeyboardStartAttack1` _player2_references)))))

(event `InputAction|Attack2P2`
  (params (Key :type "Key Structure"))
  (bind _player2_references (`self.Player2 References`))
  (:`Pressed`
    (`/Engine/EditorBlueprintResources/StandardMacros.IsValid` _player2_references
      (:`Is Valid`
        (`self.P2KeyboardStartAttack2` _player2_references)))))

(event `InputAction|Attack3P2`
  (params (Key :type "Key Structure"))
  (bind _player2_references (`self.Player2 References`))
  (:`Pressed`
    (`/Engine/EditorBlueprintResources/StandardMacros.IsValid` _player2_references
      (:`Is Valid`
        (`self.P2KeyboardStartAttack3` _player2_references)))))

(event `InputAction|Attack4P2`
  (params (Key :type "Key Structure"))
  (bind _player2_references (`self.Player2 References`))
  (:`Pressed`
    (`/Engine/EditorBlueprintResources/StandardMacros.IsValid` _player2_references
      (:`Is Valid`
        (`self.P2KeyboardStartAttack4` _player2_references)))))

(event `InputAxis|MoveRightP2`
  (params (AxisValue :type "Float (single-precision)"))
  (bind _player2_references (`self.Player2 References`))
  (`/Engine/EditorBlueprintResources/StandardMacros.IsValid` _player2_references
    (:`Is Valid`
      (`self.P2KeyboardMoveRight` _player2_references AxisValue))))

(fn `UserConstructionScript`)