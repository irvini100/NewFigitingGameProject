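; Hitbox actor for a fighting game that displays a proximity, strike or hurtbox volume and deals damage to the opposing player.
; SpawnHitBox sets the display material by type, moves and reveals the display, then runs a single collision check regardless of type.
; DeterminePlayer caches the game mode and compares the owner to Player1 to pick the opponent.
; An overlap with that opponent's Hurtbox calls TakeDamage with HitboxDamage.
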(event `Spawn HitBox`
  (switch `EHitboxEnum` (`self.hitboxType`)
    (:`HB_PROXIMITY`
      (`PrimitiveComponent.SetMaterial` (`self.HitboxDisplay`) 0 "/Game/Art/Materials/Hitboxes/HB_Proximity_Hitbox.HB_Proximity_Hitbox"))
    (:`HB_STRIKE`
      (`PrimitiveComponent.SetMaterial` (`self.HitboxDisplay`) 0 "/Game/Art/Materials/Hitboxes/HB_Strike.HB_Strike"))
    (:`HB_HURTBOX`
      (`PrimitiveComponent.SetMaterial` (`self.HitboxDisplay`) 0 "/Game/Art/Materials/Hitboxes/HB_Hurtbox.HB_Hurtbox")))
  (`SceneComponent.K2_SetWorldLocation` (`self.HitboxDisplay`) (`self.hitboxLocation`) false false)
  (`SceneComponent.SetVisibility` (`self.HitboxDisplay`) true false)
  (`self.Check Collision`))

(event `Check Collision`
  (bind _player2 (`FightingGameProjectGameMode.player2` (`self.BaseGameModeReference`)))
  (bind _player1 (`FightingGameProjectGameMode.player1` (`self.BaseGameModeReference`)))
  (bind _isplayerone (`self.DeterminePlayer`))
  (if _isplayerone
    (if (`self.IsOverlappingActor` (`FightingGameProjectCharacter.hurtbox` _player2))
      (`FightingGameProjectCharacter.TakeDamage` _player2 (`self.hitboxDamage`)))
    (elif (`self.IsOverlappingActor` (`FightingGameProjectCharacter.hurtbox` _player1))
      (`FightingGameProjectCharacter.TakeDamage` _player1 (`self.hitboxDamage`)))))

(fn `DeterminePlayer`
  (returns (IsPlayerOne :type Boolean))
  (bind _asfighting_game_project_game_mode (cast `FightingGameProjectGameMode` (`GameplayStatics.GetGameMode`)))
  (bind _output_get (set `self.BaseGameModeReference` _asfighting_game_project_game_mode))
  (if (== (`FightingGameProjectGameMode.player1` _output_get) (`self.GetOwner`))
    (return true)
    (else
      (return false))))

(fn `UserConstructionScript`)